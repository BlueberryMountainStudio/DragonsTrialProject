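; BP_Spline2 is a prototype actor that lays MagicVine meshes along an editable spline.
; The Construction Script divides the spline length by SectionLength and adds a SplineMeshComponent for each section, deforming along the X axis.
; Helper functions supply each section's local start and end positions and tangents, clamping tangent size to SectionLength.
; The event graph holds no active logic.
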(event EventBeginPlay)

(event Collision|EventActorBeginOverlap
  (params (OtherActor :type Actor%20Object%20Reference)))

(event EventTick
  (params (DeltaSeconds :type Float%20%28single-precision%29)))

(fn ConstructionScript
  (for _index (range 0 (Math|Float|Truncate (/ (Spline|GetSplineLength (Variables|Default|GetSpline)) (Variables|Spline|GetSection%20Length))))
    (Variables|Spline|SetLoop%20Index _index)
    (bind _returnvalue (AddComponent|AddSplineMeshComponent false))
    (Components|StaticMesh|SetStaticMesh _returnvalue "/Game/Assets/Temporary/MagicVine.MagicVine")
    (SplineMesh|SetForwardAxis _returnvalue "X" true)
    (bind (_position _tangent) (CallFunction|GetStartPos/Tangent (Variables|Spline|GetLoop%20Index)))
    (bind (_position_2 _tangent_2) (CallFunction|GetEndPosition/Tangent (Variables|Spline|GetLoop%20Index)))
    (SplineMesh|SetStartandEnd _returnvalue _position _tangent _position_2 _tangent_2 true :!class /Script/Engine.SplineMeshComponent)))

(fn GetStartPos/Tangent
  (params (Index :type Integer))
  (bind _spline (Variables|Default|GetSpline))
  (bind _section_length (Variables|Spline|GetSection%20Length))
  (bind _returnvalue (* Index _section_length))
  (return (Spline|GetLocationatDistanceAlongSpline _spline _returnvalue "Local") (Math|Vector|ClampVectorSize (Spline|GetTangentatDistanceAlongSpline _spline _returnvalue "Local") 0.0 (Variables|Spline|GetSection%20Length))))

(fn GetEndPosition/Tangent
  (params (Index :type Integer))
  (bind _returnvalue (+ Index 1))
  (bind _section_length (Variables|Spline|GetSection%20Length))
  (bind _spline (Variables|Default|GetSpline))
  (bind _returnvalue_2 (* _returnvalue _section_length))
  (return (Spline|GetLocationatDistanceAlongSpline _spline _returnvalue_2 "Local") (Math|Vector|ClampVectorSize (Spline|GetTangentatDistanceAlongSpline _spline _returnvalue_2 "Local") 0.0 (Variables|Spline|GetSection%20Length))))