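; BP_Enemy is an enemy actor that tracks health and destroys itself when damage brings it to zero or below.
; CurrentHealth starts at MaxHealth on BeginPlay and drops with each AnyDamage event.
; A surviving hit raises HitL, or HitR if HitL is already set, and clears the flags after a short Delay.
; The flags appear intended to drive damage animation, which is not played in this graph.
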(event EventBeginPlay
  (Variables|Default|SetCurrentHealth (Variables|Default|GetMaxHealth)))

(event Game|Damage|EventAnyDamage
  (params (Damage :type Float%20%28single-precision%29) (DamageType :type Damage%20Type%20Object%20Reference) (InstigatedBy :type Controller%20Object%20Reference) (DamageCauser :type Actor%20Object%20Reference))
  ;[1 1 1] loose health on damage taken, play damage animation and eventually destroy actor when health below 0
  (if (Variables|Damage|GetHitL)
    (Variables|Damage|SetHitR true)
    (bind _output_get (Variables|Default|SetCurrentHealth (- (Variables|Default|GetCurrentHealth) Damage)))
    (if (<= _output_get 0.0)
      (Actor|DestroyActor)
      (else
        (Utilities|FlowControl|Delay 1.0)
        (Variables|Damage|SetHitL false)
        (Variables|Damage|SetHitR false)))
    (else
      (Variables|Damage|SetHitL true)
      (bind _output_get_2 (Variables|Default|SetCurrentHealth (- (Variables|Default|GetCurrentHealth) Damage)))
      (if (<= _output_get_2 0.0)
        (Actor|DestroyActor)
        (else
          (Utilities|FlowControl|Delay 1.0)
          (Variables|Damage|SetHitL false))))))

(fn ConstructionScript)