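; Enemy character that takes damage and knockback from the player's combo attacks.
; Any overlap makes it apply damage to itself; AnyDamage ignores that amount and uses the player's ComboIndex to pick one of three damage and knockback pairs.
; A DoOnce-gated helper sets movement velocity and lowers health, followed by a health check and DestroyActor.
; Debug prints report health, damage and unmatched combo indices.
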(event EventBeginPlay
  (Variables|Default|SetCurrentHealth (Variables|Default|GetMaxHealth))
  (bind _asbp_mc (Utilities|Casting|CastToBP_MC (Game|Player|GetPlayerPawn 0)))
  (Variables|Default|SetPlayer_REF _asbp_mc)
  (bind _asbp_main_character_player_character_controller (Utilities|Casting|CastToBP_MainCharacterPlayerCharacterController (Game|GetPlayerController 0)))
  (Variables|Default|SetController_REF _asbp_main_character_player_character_controller))

(event Game|Damage|EventAnyDamage
  (params (Damage :type Float%20%28single-precision%29) (DamageType :type Damage%20Type%20Object%20Reference) (InstigatedBy :type Controller%20Object%20Reference) (DamageCauser :type Actor%20Object%20Reference))
  (bind _player_ref (Variables|Default|GetPlayer_REF))
  (bind _player_ref_2 (Variables|Default|GetPlayer_REF))
  (bind _player_ref_3 (Variables|Default|GetPlayer_REF))
  (switch int (Variables|/Game/Programming/Actors/BP_MC.BP_MC_C|GetComboIndex (Variables|Default|GetPlayer_REF))
    (:Default
      (Development|PrintString "no attack indx"))
    (:1
      (CallFunction|DamageKnockbackApply (Variables|/Game/Programming/Actors/BP_MC.BP_MC_C|GetComb1_Damage _player_ref) (Variables|/Game/Programming/Actors/BP_MC.BP_MC_C|GetComb1_Knockback _player_ref))
      (CallFunction|IsActorDead)
      (Actor|DestroyActor :!label _label))
    (:2
      (CallFunction|DamageKnockbackApply (Variables|/Game/Programming/Actors/BP_MC.BP_MC_C|GetComb2_Damage _player_ref_3) (Variables|/Game/Programming/Actors/BP_MC.BP_MC_C|GetComb2_Knockback _player_ref_3))
      (CallFunction|IsActorDead)
      (goto _label))
    (:3
      (CallFunction|DamageKnockbackApply (Variables|/Game/Programming/Actors/BP_MC.BP_MC_C|GetComb3_Damage _player_ref_2) (Variables|/Game/Programming/Actors/BP_MC.BP_MC_C|GetComb3_Knockback _player_ref_2))
      (CallFunction|IsActorDead)
      (goto _label))))

(event Collision|EventActorBeginOverlap
  (params (OtherActor :type Actor%20Object%20Reference))
  (Game|Damage|ApplyDamage self 3e+01 0 0))

(fn ConstructionScript)

(fn DecreaseHealth
  (params (Damage :type Float%20%28double-precision%29))
  (Variables|Default|SetCurrentHealth (- (Variables|Default|GetCurrentHealth) Damage)))

(fn IsActorDead
  (bind _currenthealth (Variables|Default|GetCurrentHealth))
  (Development|PrintString (Utilities|String|ToString(Float) _currenthealth))
  (if (<= _currenthealth 0.0)
    (return)
    (else
      (return))))

(fn ApplyKnockback
  (params (Knockback :type Vector))
  (Variables|/Script/Engine.MovementComponent|SetVelocity (Variables|Character|GetCharacterMovement) Knockback))

(fn CheckAttackIndex
  (params (Number :type Integer))
  (if (== Number (Variables|/Game/Programming/Game/BP_MainCharacterPlayerCharacterController.BP_MainCharacterPlayerCharacterController_C|GetAttackIndex (Variables|Default|GetController_REF)))
    (return true)
    (else
      (return false))))

(fn DamageKnockbackApply
  (params (Damage :type Float%20%28double-precision%29) (Knockback :type Vector))
  (Utilities|FlowControl|DoOnce false
    (:Completed
      (CallFunction|ApplyKnockback Knockback)
      (CallFunction|DecreaseHealth Damage)
      (Variables|Default|SetComb1 false)
      (Variables|Default|SetComb2 false)
      (Variables|Default|SetComb3 false)
      (Development|PrintString (Utilities|String|ToString(Float) Damage)))))