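; BP_MC is the player character Blueprint, handling melee combos, a dash and jump helpers.
; Attacks plays a three-montage combo, gated by DoOnce, with one-press buffering and timed reset; separate events toggle HurtboxV2 collision, while sphere-trace damage is left unwired.
; Dash plays a montage while a timeline drives forward velocity.
; Holding Space on landing re-jumps for bunny hopping; walking off ledges starts a coyote timer whose timeout is empty.
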(event Custom|CoyoteTimerOut
  ;[1 1 1] bHop
)

(event Custom|Dash
  (bind _charactermovement (Variables|Character|GetCharacterMovement))
  (Animation|Montage|PlayMontage (Variables|Character|GetMesh) "/Game/Assets/Temporary/AnimM_Bean_PZ_dash.AnimM_Bean_PZ_dash" (Variables|Movement|GetDashAnimPlayrate)
    (:then
      (Timeline|Timeline PlayFromStart
        (:Update
          (Variables|/Script/Engine.CharacterMovementComponent|SetGroundFriction _charactermovement 0.0)
          (Variables|/Script/Engine.MovementComponent|SetVelocity _charactermovement (* (Transformation|GetActorForwardVector) (Variables|Movement|GetDashDistance)))
          (Variables|/Script/Engine.CharacterMovementComponent|SetGroundFriction _charactermovement (Variables|Movement|GetFriction%20Resetter)))))))

(event Custom|Deactivate%20Mesh%20Hurtbox
  (Collision|SetCollisionEnabled (Variables|Default|GetHurtbox_V2) "NoCollision")
  (Development|PrintString (Utilities|String|ToString(Boolean) (Class|PrimitiveComponent|IsCollisionEnabled (Variables|Default|GetHurtbox_V2)))))

(event Custom|Attacks
  ;[1 1 1] Combo, ComboBuffer and ComboReset
  (if (Variables|Default|GetAnimMontagePlaying?)
    (Variables|Attacks|SetAttackBuffered? true)
    (else
      (Utilities|FlowControl|DoOnce false
        (:Completed
          (Utilities|Time|PauseTimerbyHandle (Variables|Attacks|GetComboResetHandle))
          (bind _result (Math|Integer|IncrementInt (Variables|Attacks|GetComboIndex))
            (:%20%20
              (switch int _result
                (:1
                  (Variables|Default|SetAnimMontagePlaying? true)
                  (Animation|Montage|PlayMontage (Variables|Character|GetMesh) "/Game/Assets/Temporary/BM_Combo1.BM_Combo1"
                    (:OnCompleted
                      (bind _returnvalue (Utilities|Time|SetTimerbyEvent (delegate Custom|ComboReset) (Variables|Attacks|GetTimeUntilComboReset)))
                      (Variables|Attacks|SetComboResetHandle _returnvalue)
                      (Variables|Default|SetAnimMontagePlaying? false)
                      (CallFunction|ResetAttack)
                      (if (Variables|Attacks|GetAttackBuffered?)
                        (CallFunction|Attacks)
                        (Variables|Attacks|SetAttackBuffered? false)))))
                (:2
                  (Variables|Default|SetAnimMontagePlaying? true)
                  (Animation|Montage|PlayMontage (Variables|Character|GetMesh) "/Game/Assets/Temporary/BM_Combo2.BM_Combo2"
                    (:OnCompleted
                      (bind _returnvalue_2 (Utilities|Time|SetTimerbyEvent (delegate Custom|ComboReset) (Variables|Attacks|GetTimeUntilComboReset)))
                      (Variables|Attacks|SetComboResetHandle _returnvalue_2)
                      (Variables|Default|SetAnimMontagePlaying? false)
                      (CallFunction|ResetAttack)
                      (if (Variables|Attacks|GetAttackBuffered?)
                        (CallFunction|Attacks)
                        (Variables|Attacks|SetAttackBuffered? false)))))
                (:3
                  (Variables|Default|SetAnimMontagePlaying? true)
                  (Animation|Montage|PlayMontage (Variables|Character|GetMesh) "/Game/Assets/Temporary/BM_Combo3.BM_Combo3"
                    (:OnCompleted
                      (bind _returnvalue_3 (Utilities|Time|SetTimerbyEvent (delegate Custom|ComboReset) (Variables|Attacks|GetTimeUntilComboReset)))
                      (Variables|Attacks|SetComboResetHandle _returnvalue_3)
                      (Variables|Default|SetAnimMontagePlaying? false)
                      (Variables|Attacks|SetComboIndex 0)
                      (CallFunction|ResetAttack)
                      (if (Variables|Attacks|GetAttackBuffered?)
                        (CallFunction|Attacks)
                        (Variables|Attacks|SetAttackBuffered? false)))))))))))))

(event Custom|Reset%20Attack
  ;[1 1 1] Combo, ComboBuffer and ComboReset
  (Utilities|FlowControl|DoOnce false) ; enters at Reset
)

(event Custom|Trace%20Hurtbox%20Comb%203
  ;[1 1 1] Trace Hurtboxes for Combo Attack (activated in ABP_MC)
)

(event Custom|ComboReset
  ;[1 1 1] Combo, ComboBuffer and ComboReset
  (Variables|Attacks|SetComboIndex 0))

(event Custom|TraceHurtbox_Comb1
  (params (Y-Achse :type Float%20%28double-precision%29))
  ;[1 1 1] Trace Hurtboxes for Combo Attack (activated in ABP_MC)
)

(event Custom|Activate%20Mesh%20Hurtbox
  (Collision|SetCollisionEnabled (Variables|Default|GetHurtbox_V2) "QueryAndPhysics")
  (Development|PrintString (Utilities|String|ToString(Boolean) (Class|PrimitiveComponent|IsCollisionEnabled (Variables|Default|GetHurtbox_V2)))))

(event Custom|Trace%20Hurtbox%20Comb%202
  ;[1 1 1] Trace Hurtboxes for Combo Attack (activated in ABP_MC)
)

(event Custom|Check%20Hurtbox%20Active
  (Development|PrintString (Utilities|String|ToString(Boolean) (Class|PrimitiveComponent|IsCollisionEnabled (Variables|Default|GetHurtbox_V2)))))

(event EventBeginPlay
  (Collision|SetCollisionEnabled (Variables|Default|GetHurtbox_V2) "NoCollision"))

(event EventOnMovementModeChanged
  (params (PrevMovementMode :type EMovementMode%20Enum :default "MOVE_None") (NewMovementMode :type EMovementMode%20Enum :default "MOVE_None") (PrevCustomMode :type Byte :default 0) (NewCustomMode :type Byte :default 0))
  ;[1 1 1] Bunny Hop
  (if (Utilities|Enum|Equal(Enum) NewMovementMode "MOVE_Walking")
    (bind _asbp_main_character_player_character_controller (Utilities|Casting|CastToBP_MainCharacterPlayerCharacterController (Game|GetPlayerController 0)))
    (if (Game|Player|IsInputKeyDown _asbp_main_character_player_character_controller "SpaceBar")
      (Character|Jump))
    (else
      ;[1 1 1] bHop
      (if (and (Utilities|Enum|Equal(Enum) PrevMovementMode "MOVE_Walking") (Utilities|Enum|Equal(Enum) NewMovementMode "MOVE_Falling"))
        (bind _returnvalue (Utilities|Time|SetTimerbyEvent (delegate Custom|CoyoteTimerOut) (Variables|Movement|GetCoyote%20Time)))
        (Variables|Movement|SetCoyote%20Timer _returnvalue)))))

(event EventOnLanded
  (params (Hit :type Hit%20Result%20Structure%20%28by%20ref%29))
  ;[1 1 1] bHop
  (Utilities|Time|ClearandInvalidateTimerbyHandle (Variables|Movement|GetCoyote%20Timer))
  (bind _asbp_main_character_player_character_controller (Utilities|Casting|CastToBP_MainCharacterPlayerCharacterController (Game|GetPlayerController 0)))
  (Variables|/Game/Programming/Game/BP_MainCharacterPlayerCharacterController.BP_MainCharacterPlayerCharacterController_C|SetIsLanded _asbp_main_character_player_character_controller true))

(fn ConstructionScript)

(fn TraceHurtboxbySphere
  (params (Y-Richtung :type Float%20%28double-precision%29) (Range :type Float%20%28double-precision%29) (Radius :type Float%20%28single-precision%29) (BaseDamage :type Float%20%28single-precision%29))
  (bind _returnvalue (Game|GetPlayerCharacter 0))
  (bind _returnvalue_2 (Transformation|GetActorLocation _returnvalue))
  (bind _outhit (Collision|SphereTraceByChannel (+ _returnvalue_2 "0.000000,100.000000,0.000000") (+ _returnvalue_2 (* (Math|Vector|MakeVector 0.0 (Math|Float|Clamp(Float) Y-Richtung -1.0) 0.0) Range)) Radius "TraceTypeQuery3" true 0 "Persistent")))