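; Player character Blueprint that adds bunny hopping and the beginnings of coyote time.
; Landing into walking while Space is held triggers an immediate jump.
; Walking into falling starts a coyote timer whose timeout handler is empty; landing clears a timer handle.
; Tick restores ground friction to its BeginPlay value whenever absolute Y velocity is within max walk speed, though nothing here changes it otherwise.
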(event Custom|CoyoteTimerOut
  ;[1 1 1] bHop
)

(event EventBeginPlay
  (Variables|Default|SetFriction%20Resetter (Variables|/Script/Engine.CharacterMovementComponent|GetGroundFriction (Variables|Character|GetCharacterMovement))))

(event EventTick
  (params (DeltaSeconds :type Float%20%28single-precision%29))
  (bind _charactermovement (Variables|Character|GetCharacterMovement))
  (if (<= (Math|Float|Absolute(Float) (.y (Transformation|GetVelocity))) (Variables|/Script/Engine.CharacterMovementComponent|GetMaxWalkSpeed _charactermovement))
    (Variables|/Script/Engine.CharacterMovementComponent|SetGroundFriction _charactermovement (Variables|Default|GetFriction%20Resetter))))

(event EventOnMovementModeChanged
  (params (PrevMovementMode :type EMovementMode%20Enum :default "MOVE_None") (NewMovementMode :type EMovementMode%20Enum :default "MOVE_None") (PrevCustomMode :type Byte :default 0) (NewCustomMode :type Byte :default 0))
  ;[1 1 1] Bunny Hop
  (if (Utilities|Enum|Equal(Enum) NewMovementMode "MOVE_Walking")
    (bind _asbp_main_character_player_character_controller (Utilities|Casting|CastToBP_MainCharacterPlayerCharacterController (Game|GetPlayerController 0)))
    (if (Game|Player|IsInputKeyDown _asbp_main_character_player_character_controller "SpaceBar")
      (Character|Jump))
    (else
      ;[1 1 1] bHop
      (if (and (Utilities|Enum|Equal(Enum) PrevMovementMode "MOVE_Walking") (Utilities|Enum|Equal(Enum) NewMovementMode "MOVE_Falling"))
        (bind _returnvalue (Utilities|Time|SetTimerbyEvent (delegate Custom|CoyoteTimerOut) (Variables|Default|GetCoyote%20Time)))
        (Variables|Default|SetCoyote%20Timer _returnvalue)))))

(event EventOnLanded
  (params (Hit :type Hit%20Result%20Structure%20%28by%20ref%29))
  ;[1 1 1] bHop
  (Utilities|Time|ClearandInvalidateTimerbyHandle (Variables|Default|GetCoyete%20Timer)))

(fn ConstructionScript)