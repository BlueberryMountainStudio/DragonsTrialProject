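; Actor Blueprint that plays a mood theme song and pulses a sphere to the music's loudness.
; The construction script caches the sound's duration from an analyzer asset.
; On audio playback percent updates, it converts the percent to seconds, samples channel-zero loudness at that time, and sets the sphere's uniform scale to that value.
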(event Custom|CustomEvent
  (params (PlayingSoundWave :type Sound%20Wave%20Object%20Reference) (PlaybackPercent :type Float%20%28single-precision%29))
  (Transformation|SetRelativeScale3D (Variables|Default|GetSphere) (Math|Conversions|ToVector(Float) (Class|LoudnessNRT|GetChannelLoudnessatTime (Variables|Default|GetNewVar) (* PlaybackPercent (Variables|Default|GetNewVar_0))))))

(event EventBeginPlay
  (EventDispatchers|BindEventtoOnAudioPlaybackPercent (Variables|Default|GetAudio) (delegate Custom|CustomEvent)))

(event Collision|EventActorBeginOverlap
  (params (OtherActor :type Actor%20Object%20Reference)))

(event EventTick
  (params (DeltaSeconds :type Float%20%28single-precision%29)))

(fn ConstructionScript
  (Variables|Default|SetNewVar_0 (Variables|/Script/Engine.SoundBase|GetDuration (Variables|/Script/AudioAnalyzer.AudioAnalyzerNRT|GetSound (Variables|Default|GetNewVar)))))