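; MainTheme is an actor that drives the main theme's audio component through float parameters.
; It sets BPM to a calm default at start, raises it while an actor begins overlapping and restores it on end overlap.
; Handlers forward MIDI notes to a "MIDI In" parameter and raise the actor on higher-numbered control changes, but the MIDI device setup binding them is disconnected, so never runs.
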(event Custom|OnActorEndOverlap_Event
  (params (OverlappedActor :type Actor%20Object%20Reference) (OtherActor :type Actor%20Object%20Reference))
  (Audio|Parameter|SetFloatParameter (Variables|Default|GetAudio) "BPM" 9e+01 :!class /Script/Engine.AudioComponent))

(event Custom|PlayNote
  (params (MIDIDeviceController :type MIDI%20Device%20Input%20Controller%20Object%20Reference) (Timestamp :type Integer) (Channel :type Integer) (Note :type Integer) (Velocity :type Integer))
  (Audio|Parameter|SetFloatParameter (Variables|Default|GetAudio) "MIDI In" (Math|Conversions|ToFloat(Integer) Note) :!class /Script/Engine.AudioComponent))

(event Custom|ChangeControl
  (params (MIDIDeviceController :type MIDI%20Device%20Input%20Controller%20Object%20Reference) (Timestamp :type Integer) (Channel :type Integer) (Type :type Integer) (Value :type Integer))
  (Math|Integer|CompareInt Type 70
    (:>
      (Transformation|SetActorLocation (Math|Vector|MakeVector 0.0 0.0 (+ (.z (Transformation|GetActorLocation)) (Math|Conversions|ToFloat(Integer) Value))) true false))))

(event EventBeginPlay
  (Audio|Parameter|SetFloatParameter (Variables|Default|GetAudio) "BPM" 9e+01 :!class /Script/Engine.AudioComponent)
  (EventDispatchers|BindEventtoOnActorEndOverlap (delegate Custom|OnActorEndOverlap_Event)))

(event Collision|EventActorBeginOverlap
  (params (OtherActor :type Actor%20Object%20Reference))
  (Audio|Parameter|SetFloatParameter (Variables|Default|GetAudio) "BPM" 1.6e+02 :!class /Script/Engine.AudioComponent))

(event EventTick
  (params (DeltaSeconds :type Float%20%28single-precision%29)))

(fn ConstructionScript)