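; Enemy with health that takes damage and knockback from the player's three-step combo, stored in a folder marked as outdated and slated for deletion.
; BeginPlay caches the player pawn and controller and fills health to maximum.
; AnyDamage picks a knockback vector by the player's ComboIndex, writes it to FloatingPawnMovement velocity, subtracts health and destroys the actor at zero or below.
; CheckAttackIndex compares against the controller's AttackIndex but is never called here.
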(event EventBeginPlay
  (bind _asbp_mc (Utilities|Casting|CastToBP_MC (Game|Player|GetPlayerPawn 0)))
  (Variables|Default|SetPlayer_REF _asbp_mc)
  (bind _asbp_main_character_player_character_controller (Utilities|Casting|CastToBP_MainCharacterPlayerCharacterController (Game|GetPlayerController 0)))
  (Variables|Default|SetController_REF _asbp_main_character_player_character_controller)
  (Variables|Default|SetCurrentHealth (Variables|Default|GetMaxHealth)))

(event Game|Damage|EventAnyDamage
  (params (Damage :type Float%20%28single-precision%29) (DamageType :type Damage%20Type%20Object%20Reference) (InstigatedBy :type Controller%20Object%20Reference) (DamageCauser :type Actor%20Object%20Reference))
  (switch int (Variables|/Game/Programming/Actors/BP_MC.BP_MC_C|GetComboIndex (Variables|Default|GetPlayer_REF))
    (:1
      (CallFunction|DamageKnockbackAttack (Variables|/Game/Programming/Actors/BP_MC.BP_MC_C|GetComb1_Knockback (Variables|Default|GetPlayer_REF)) Damage))
    (:2
      (CallFunction|DamageKnockbackAttack (Variables|/Game/Programming/Actors/BP_MC.BP_MC_C|GetComb2_Knockback (Variables|Default|GetPlayer_REF)) Damage))
    (:3
      (CallFunction|DamageKnockbackAttack (Variables|/Game/Programming/Actors/BP_MC.BP_MC_C|GetComb3_Knockback (Variables|Default|GetPlayer_REF)) Damage)))
  (bind _dead (CallFunction|IsActorDead?))
  (if _dead
    (Actor|DestroyActor)))

(fn ConstructionScript)

(fn ApplyKnockback
  (params (Knockback%20Vector :type Vector))
  (Variables|/Script/Engine.MovementComponent|SetVelocity (Variables|Default|GetFloatingPawnMovement) Knockback%20Vector))

(fn DecreaseHealth
  (params (Icoming%20Damage :type Float%20%28double-precision%29))
  (Variables|Default|SetCurrentHealth (- (Variables|Default|GetCurrentHealth) Icoming%20Damage)))

(fn IsActorDead?
  (if (<= (Variables|Default|GetCurrentHealth) 0.0)
    (return true)
    (else
      (return false))))

(fn CheckAttackIndex
  (params (Index%20in%20Question :type Integer))
  (if (== Index%20in%20Question (Variables|/Game/Programming/Game/BP_MainCharacterPlayerCharacterController.BP_MainCharacterPlayerCharacterController_C|GetAttackIndex (Variables|Default|GetController_REF)))
    (return true)
    (else
      (return false))))

(fn DamageKnockbackAttack
  (params (Knockback%20Vector :type Vector) (Icoming%20Damage :type Float%20%28double-precision%29))
  (Utilities|FlowControl|DoOnce false
    (:Completed
      (CallFunction|ApplyKnockback Knockback%20Vector)
      (CallFunction|DecreaseHealth Icoming%20Damage)
      (Variables|Default|SetHitComb1 false)
      (Variables|Default|SetHitComb2 false)
      (Variables|Default|SetHitComb3 false)
      (Development|PrintString (Utilities|String|ToString(Float) Icoming%20Damage)))))